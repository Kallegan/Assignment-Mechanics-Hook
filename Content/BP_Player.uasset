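; Player Blueprint that plays footstep and landing sounds that vary with the surface underfoot.
; A looping timer created paused at BeginPlay fires footsteps, with PlayFootstepsSFX unpausing it while the player moves without vertical velocity and pausing it otherwise.
; Footsteps and OnLanded spawn sounds below the actor's origin.
; A downward trace treats BP_AttachableActorBase hits as metal, setting each sound's "Material" parameter.
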(event `self.ReceiveBeginPlay`
  (`parent.ReceiveBeginPlay`)
  (bind _returnvalue (`KismetSystemLibrary.K2_SetTimer` null "PlayFootstepSFX" 0.4 true))
  (bind _output_get (set `self.FootstepTimerhandle` _returnvalue))
  (`KismetSystemLibrary.K2_PauseTimerHandle` _output_get))

(event `self.K2_PlayFootstepsSFX`
  (bind (_returnvalue_x _returnvalue_y _returnvalue_z) (`KismetMathLibrary.BreakVector` (`self.GetVelocity`)))
  (bind _footsteptimerhandle (`self.FootstepTimerhandle`))
  (if (and (== _returnvalue_z 0.0) (> (`KismetMathLibrary.VSize` (`self.GetVelocity`)) 0.0))
    (`KismetSystemLibrary.K2_UnPauseTimerHandle` _footsteptimerhandle)
    (else
      (`KismetSystemLibrary.K2_PauseTimerHandle` _footsteptimerhandle))))

(event `self.OnLanded`
  (params (Hit :type "HitResult Structure (by ref)"))
  (`parent.OnLanded` Hit)
  (`self.PlayLandingSFX`))

(fn `PlayFootstepSFX`
  (locals (NewLocalVar :type "SoundBase Object Reference" :default "/Script/Engine.SoundCue'/Game/SFX/Footsteps/SC_Walk.SC_Walk'"))
  (bind (_returnvalue_x _returnvalue_y _returnvalue_z) (`KismetMathLibrary.BreakVector` (`self.GetVelocity`)))
  (if (and (== _returnvalue_z 0.0) (> (`KismetMathLibrary.VSize` (`self.GetVelocity`)) 0.0))
    (bind _returnvalue (`GameplayStatics.SpawnSoundAtLocation` "/Game/SFX/Footsteps/SC_Walk.SC_Walk" (- (`self.K2_GetActorLocation`) (0.0 0.0 44.0)) (struct) 1.0 1.0 0.0 null null))
    (bind _returnvalue_2 (`self.TraceForMetalSurface`))
    (`AudioComponent.SetIntParameter` _returnvalue "Material" (`KismetMathLibrary.Conv_BoolToInt` _returnvalue_2))
    (else
      (`KismetSystemLibrary.K2_PauseTimerHandle` (`self.FootstepTimerhandle`)))))

(fn `PlayLandingSFX`
  (bind _returnvalue (`GameplayStatics.SpawnSoundAtLocation` "/Game/SFX/Footsteps/SC_Land.SC_Land" (- (`self.K2_GetActorLocation`) (0.0 0.0 44.0)) (struct) 1.0 1.0 0.0 null null))
  (bind _returnvalue_2 (`self.TraceForMetalSurface`))
  (`AudioComponent.SetIntParameter` _returnvalue "Material" (`KismetMathLibrary.Conv_BoolToInt` _returnvalue_2)))

(fn `TraceForMetalSurface`
  (returns (ReturnValue :type Boolean))
  (bind _returnvalue (`self.K2_GetActorLocation`))
  (bind _outhit (`KismetSystemLibrary.LineTraceSingle` _returnvalue (- _returnvalue (0.0 0.0 200.0)) "TraceTypeQuery1"))
  (return (`GameplayStatics.ObjectIsA` (`.HitActor` (`GameplayStatics.BreakHitResult` _outhit)) "/Game/Blueprints/Actors/InteractableActor/BP_AttachableActorBase.BP_AttachableActorBase_C")))

(fn `UserConstructionScript`
  (`parent.UserConstructionScript`))