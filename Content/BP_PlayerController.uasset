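; Player controller for first-person projectile recall and teleport-style movement, plus checkpoint respawn and a room-switch cheat.
; A looping timer sphere-traces from the camera and stores the interactable actor it returns.
; Right-click recalls all projectiles; Tick pulls the character via LaunchCharacter toward the stored actor while it is an attached projectile.
; TraceProjectilePath, uncalled here, predicts a near-zero-gravity path with one bounce; the Interact graph is dead.
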(event `self.ReceiveBeginPlay`
  (bind _ascharacter (cast `Character` (`self.K2_GetPawn`)))
  (set `self.PlayerCharacterRef` _ascharacter)
  (`KismetSystemLibrary.K2_SetTimer` null "Interacting" (`InteractData.InteractUpdateTime` (`self.InteractData`)) true))

(event `Key|RightMouseButton`
  (params (Key :type "Key Structure"))
  (:`Pressed`
    (set `self.bRecalled` false)
    (bind _outactors (`GameplayStatics.GetAllActorsOfClass` "/Game/Blueprints/Actors/BP_FirstPersonProjectile.BP_FirstPersonProjectile_C"))
    (if (> (`KismetArrayLibrary.Array_Length` _outactors) 0)
      (for _array_element _outactors
        (`/Game/Blueprints/Actors/BP_FirstPersonProjectile.RecallAction` _array_element)
        (set `self.bRecalled` true))
      (if (`self.bRecalled`)
        (`/Engine/EditorBlueprintResources/StandardMacros.DoOnce` false :!label _label
          (:`Completed`
            (`GameplayStatics.PlaySound2D` "/Engine/VREditor/Sounds/UI/Teleport_Mode_Entered.Teleport_Mode_Entered" 1.0 1.0 0.0 null null)
            (`KismetSystemLibrary.Delay` 1.0)
            (goto _label :!via `Reset`)))))))

(event `self.ReceiveTick`
  (params (DeltaSeconds :type "Float (single-precision)"))
  (bind _playercharacterref (`self.PlayerCharacterRef`))
  (bind (_returnvalue_x _returnvalue_y _returnvalue_z) (`KismetMathLibrary.BreakVector` (`self.K2_GetActorLocation` (`self.PlayerCharacterRef`))))
  (bind (_returnvalue_x_2 _returnvalue_y_2) (`KismetMathLibrary.BreakVector` (* (`KismetMathLibrary.Normal` (`self.GetActorForwardVector` _playercharacterref)) 150)))
  (bind _interactactor (`self.InteractActor`)
    (:`then`
      (bind _asbp_first_person_projectile (cast `/Game/Blueprints/Actors/BP_FirstPersonProjectile` _interactactor))
      (if (`/Game/Blueprints/Actors/BP_FirstPersonProjectile.bAttached` _asbp_first_person_projectile)
        (bind (_returnvalue_x_3 _returnvalue_y_3 _returnvalue_z_2) (`KismetMathLibrary.BreakVector` (`self.K2_GetActorLocation` _interactactor)))
        (`Character.LaunchCharacter` (`self.PlayerCharacterRef`) (* (- (`self.K2_GetActorLocation` _interactactor) (- (`self.K2_GetActorLocation` _playercharacterref) (`KismetMathLibrary.MakeVector` _returnvalue_x_2 _returnvalue_y_2 (`KismetMathLibrary.FClamp` (- _returnvalue_z_2 _returnvalue_z) 0.0 500.0)))) (* (`GameplayStatics.GetWorldDeltaSeconds`) 200.0)) true true)
        (bind _result (`/Engine/EditorBlueprintResources/StandardMacros.IncrementInt` (`self.NewVar`))
          (:`  `
            (if (> _result 10)
              (set `self.NewVar` 0))))))
    (:`else`)))

(event `Key|ö`
  (params (Key :type "Key Structure"))
  (:`Pressed`
    (message `/Game/Blueprints/Interfaces/BPI_GameMode.RespawnCurrentCheckpoint` (`GameplayStatics.GetGameMode`) false)))

(event `self.DebugRoom`
  (params (RoomIndex :type Integer))
  (bind _outactors (`GameplayStatics.GetAllActorsWithInterface` "/Game/Blueprints/Interfaces/BPI_LevelInterface.BPI_LevelInterface_C"))
  (message `/Game/Blueprints/Interfaces/BPI_LevelInterface.ChangeRoom` (`|GetArrayItem` _outactors) RoomIndex))

(fn `Interact`)

(fn `Interacting`
  (bind _playercameramanager (`self.PlayerCameraManager`))
  (bind _returnvalue (`PlayerCameraManager.GetCameraLocation` _playercameramanager))
  (bind _outhit (`KismetSystemLibrary.SphereTraceSingle` :`Start` (+ _returnvalue (`KismetMathLibrary.GreaterGreater_VectorRotator` (60.0 30.0 -15.0) (`PlayerCameraManager.GetCameraRotation` _playercameramanager))) :`End` (+ _returnvalue (* (`self.GetActorForwardVector` _playercameramanager) 5000.0)) :`Radius` 20.0 :`TraceChannel` "TraceTypeQuery1" :`bTraceComplex` true :`TraceColor` (struct :`R` 0.988287 :`B` 1.0 :`A` 1.0) :`TraceHitColor` (struct :`R` 1.0 :`G` 0.632953 :`A` 1.0) :`DrawTime` (`InteractData.InteractUpdateTime` (`self.InteractData`))))
  (bind (_bblockinghit _binitialoverlap _time _distance _location _impactpoint _normal _impactnormal _physmat _hitactor _hitcomponent) (`GameplayStatics.BreakHitResult` _outhit))
  (if _bblockinghit
    (bind _returnvalue_2 (`ActorComponent.GetOwner` _hitcomponent))
    (if (`KismetSystemLibrary.DoesImplementInterface` _returnvalue_2 "/Game/Blueprints/Interfaces/BPI_Interactable.BPI_Interactable_C")
      (bind _interactactor (message `/Game/Blueprints/Interfaces/BPI_Interactable.Interacting` _returnvalue_2 (`InteractData.InteractUpdateTime` (`self.InteractData`))))
      (`/Engine/EditorBlueprintResources/StandardMacros.IsValid` _interactactor
        (:`Is Valid`
          (set `self.InteractActor` _interactactor))))))

(fn `TraceProjectilePath`
  (params (StartPos :type "Vector Structure") (CurrentVelocity :type "Vector Structure") (`Pr Radius` :type "Float (double-precision)") (`Sim TIme` :type "Float (double-precision)"))
  (returns (`Local Final Points1` :type "Array of Vector Structure"))
  (locals (`Local Current Velocity` :type "Vector Structure") (`Local Pr Radius` :type "Float (single-precision)") (`Local Sim Time` :type "Float (single-precision)") (`Local Final Points` :type "Array of Vector Structure"))
  (set `local.Local Current Velocity` CurrentVelocity)
  (set `local.Local Pr Radius` `Pr Radius`)
  (set `local.Local Sim Time` `Sim TIme`)
  (`|ExecutionSequence`
    (:`then_0`
      (bind (_outhit _outpathpositions _outlasttracedestination _returnvalue) (`GameplayStatics.Blueprint_PredictProjectilePath_ByObjectType` :`StartPos` StartPos :`LaunchVelocity` (`local.Local Current Velocity`) :`ProjectileRadius` (`local.Local Pr Radius`) :`ObjectTypes` (`|MakeArray` "ObjectTypeQuery1" :!type "EObjectTypeQuery Enum") :`DrawDebugType` "ForDuration" :`DrawDebugTime` 0.1 :`SimFrequency` 1.0 :`MaxSimTime` (`local.Local Sim Time`) :`OverrideGravityZ` 1e-06))
      (`KismetArrayLibrary.Array_Append` (`local.Local Final Points`) _outpathpositions)
      (bind _output_get (set `self.currentHit` _returnvalue))
      (if _output_get
        (set `self.currentBounceHit` (`|GetArrayItem` _outpathpositions (`KismetArrayLibrary.Array_LastIndex` _outpathpositions)))
        (bind (_bblockinghit _binitialoverlap _time _distance _location _impactpoint _normal _impactnormal _physmat _hitactor) (`GameplayStatics.BreakHitResult` _outhit))
        (set `self.currentImpactNormal` _impactnormal)
        (set `local.Local Current Velocity` (`KismetMathLibrary.MirrorVectorByNormal` (* (`local.Local Current Velocity`) 0.3) (`self.currentImpactNormal`)))
        (bind (_outhit_2 _outpathpositions_2 _outlasttracedestination_2 _returnvalue_2) (`GameplayStatics.Blueprint_PredictProjectilePath_ByObjectType` (`self.currentBounceHit`) (`local.Local Current Velocity`) true (`local.Local Pr Radius`) (`|MakeArray` "ObjectTypeQuery1" :!type "EObjectTypeQuery Enum") false (`|MakeArray` _hitactor) "ForDuration" 0.1 1.0 (`local.Local Sim Time`) 1e-06))
        (`KismetArrayLibrary.Array_Append` (`local.Local Final Points`) _outpathpositions_2)
        (if _returnvalue_2
          (bind (_bblockinghit_2 _binitialoverlap_2 _time_2 _distance_2 _location_2 _impactpoint_2 _normal_2) (`GameplayStatics.BreakHitResult` _outhit_2))
          (set `self.currentBounceHit` _location_2)
          (set `self.currentImpactNormal` _normal_2))))
    (:`then_1`
      (return (`local.Local Final Points`)))))

(fn `UserConstructionScript`)