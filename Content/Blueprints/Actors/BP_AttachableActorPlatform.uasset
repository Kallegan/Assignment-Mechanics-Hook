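; BP_AttachableActorPlatform is a child Blueprint, by name a platform variant of an attachable actor.
; It adds no logic of its own: BeginPlay, the construction script, GetProjectileRef, Interacting and IsProjectileAttachableSurface all forward to the parent.
; Projectile attachment and interaction behavior therefore come entirely from the parent class.
; Tick and overlap events are disabled placeholders.
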(event `self.ReceiveBeginPlay`
  (`parent.ReceiveBeginPlay`))

(fn `GetProjectileRef`
  (returns (ProjectileRef :type "Actor Object Reference"))
  (bind _projectileref (`parent.GetProjectileRef`))
  (return _projectileref))

(fn `Interacting`
  (params (UpdateRate :type "Float (double-precision)"))
  (returns (InteractActor :type "Actor Object Reference") (bInRange :type Boolean))
  (bind (_interactactor _binrange) (`parent.Interacting` UpdateRate))
  (return _interactactor _binrange))

(fn `IsProjectileAttachableSurface`
  (returns (bAttachable :type Boolean))
  (bind _battachable (`parent.IsProjectileAttachableSurface`))
  (return _battachable))

(fn `UserConstructionScript`
  (`parent.UserConstructionScript`))