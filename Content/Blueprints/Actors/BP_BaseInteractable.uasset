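; Base interactable actor that activates once after being interacted with for a set interaction time.
; Each Interacting call subtracts the update rate from a countdown and feeds clamped 0-to-1 progress to an emissive material component.
; When the countdown runs out, it sets Activated and calls ObjectActivated; stopping earlier resets both the timer and the emissive component's interaction.
; GetDynamicMaterial is empty here.
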(event `self.ReceiveBeginPlay`
  (set `self.CurrentInteractionTime` (`self.InteractionTime`)))

(event `/Game/Blueprints/Interfaces/BPI_Interactable.StopInteract`
  (if (not (`self.bActivated`))
    (set `self.CurrentInteractionTime` (`self.InteractionTime`))
    (`/Game/Blueprints/Components/C-EmissiveMaterialComponent.StopInteracting` (`self.C-EmissiveMaterialComponent`))))

(fn `GetDynamicMaterial`
  (returns (NewParam :type "MaterialInstanceDynamic Object Reference"))
  (return null))

(fn `Interacting`
  (params (UpdateRate :type "Float (double-precision)"))
  (returns (InteractActor :type "Actor Object Reference"))
  (if (not (`self.bActivated`))
    (bind _output_get (set `self.CurrentInteractionTime` (- (`self.CurrentInteractionTime`) UpdateRate)))
    (`/Game/Blueprints/Components/C-EmissiveMaterialComponent.Interacting` (`self.C-EmissiveMaterialComponent`) (`KismetMathLibrary.FClamp` (+ (* (/ (`self.CurrentInteractionTime`) (`self.InteractionTime`)) -1.0) 1.0)))
    (if (<= _output_get 0.0)
      (set `self.bActivated` true)
      (`self.ObjectActivated`))
    (return self)))

(fn `UserConstructionScript`)