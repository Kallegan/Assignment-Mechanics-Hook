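; BP_AttachableActorBase is a base actor for surfaces that first-person projectiles can attach to, reporting itself as an attachable surface.
; It stores a projectile reference, set directly or when a BP_FirstPersonProjectile hits its static mesh.
; Interacting gets the range check from CInteractComponent and returns the stored projectile, rather than itself, as the interact actor.
; Hover state is forwarded to CEmissiveMaterialComponent.
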(event `/Game/Blueprints/Interfaces/BPI_AttachInterface.SetProjectileReference`
  (params (ProjectileRef :type "Actor Object Reference"))
  (set `self.ProjectileRef` ProjectileRef))

(event `self.StaticMesh.OnComponentHit`
  (params (HitComponent :type "PrimitiveComponent Object Reference") (OtherActor :type "Actor Object Reference") (OtherComp :type "PrimitiveComponent Object Reference") (NormalImpulse :type "Vector Structure") (Hit :type "HitResult Structure (by ref)"))
  (if (`GameplayStatics.ObjectIsA` OtherActor "/Game/Blueprints/Actors/BP_FirstPersonProjectile.BP_FirstPersonProjectile_C")
    (set `self.ProjectileRef` OtherActor)))

(event `/Game/Blueprints/Interfaces/BPI_Interactable.HoverInteractable`
  (params (bHovered :type Boolean))
  (`/Game/Blueprints/Components/C-EmissiveMaterialComponent.SetHovered` (`self.C-EmissiveMaterialComponent`) bHovered))

(fn `GetProjectileRef`
  (returns (ProjectileRef :type "Actor Object Reference"))
  (return (`self.ProjectileRef`)))

(fn `Interacting`
  (params (UpdateRate :type "Float (double-precision)"))
  (returns (InteractActor :type "Actor Object Reference") (bInRange :type Boolean))
  (bind _binrange (`/Game/Blueprints/Components/C-InteractComponent.UpdateInteracting` (`self.C-InteractComponent`) UpdateRate))
  (return (`self.ProjectileRef`) _binrange))

(fn `IsProjectileAttachableSurface`
  (returns (bAttachable :type Boolean))
  (return true))

(fn `UserConstructionScript`)