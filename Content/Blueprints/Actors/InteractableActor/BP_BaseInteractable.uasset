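; Base interactable actor that activates after the interaction timer runs out while in range.
; Interacting takes progress from CInteractComponent, feeds it to the emissive material component and scales the point light's intensity and radius from values cached at BeginPlay.
; On completion, activation requires CanBeActivated, and BP_ActivasionArtifact objects also need a positive looted-orb value from the player state.
; Leaving range or already being activated stops the interaction.
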(event `self.ReceiveBeginPlay`
  (bind _pointlight (`self.PointLight`)
    (:`then`
      (set `self.StartIntensity` (`LightComponentBase.Intensity` _pointlight))
      (set `self.Attenuation Radius` (`LocalLightComponent.AttenuationRadius` _pointlight)))
    (:`else`)))

(event `UpdateInteractingLighting`
  (params (Percent :type "Float (double-precision)"))
  (bind _returnvalue (+ Percent 1.0))
  (bind _pointlight (`self.PointLight`))
  (if (> Percent 0.0)
    (`LightComponent.SetIntensity` _pointlight (* (`self.StartIntensity`) _returnvalue))
    (`LocalLightComponent.SetAttenuationRadius` _pointlight (* (`self.Attenuation Radius`) _returnvalue))))

(fn `Interacting`
  (params (UpdateRate :type "Float (double-precision)"))
  (returns (InteractActor :type "Actor Object Reference") (bInRange :type Boolean))
  (locals (LocalPercent :type "Float (double-precision)" :default 0.0))
  (bind (_binrange _percent _timeremaining) (`/Game/Blueprints/Components/C-InteractComponent.UpdateInteracting` (`self.C-InteractComponent`) UpdateRate))
  (set `local.LocalPercent` _percent)
  (if (and _binrange (not (`self.bActivated`)))
    (`/Game/Blueprints/Components/C-EmissiveMaterialComponent.Interacting` (`self.C-EmissiveMaterialComponent`) (`local.LocalPercent`))
    (if (<= _timeremaining 0.0)
      (if (`self.IsActivatable`)
        (set `self.bActivated` true)
        (`self.ObjectActivated`))
      (else
        (`self.UpdateInteractingLighting` (`local.LocalPercent`))))
    (return self true)
    (else
      (`/Game/Blueprints/Interfaces/BPI_Interactable.StopInteract`)
      (return null false))))

(fn `IsActivatable`
  (returns (bCanBeActivated :type Boolean))
  (bind _returnvalue (message `PlayerStateInterface.GetLootedOrbs` (`GameplayStatics.GetPlayerState` 0)))
  (return (and (or (> _returnvalue 0) (not (`GameplayStatics.ObjectIsA` self "/Game/Blueprints/Actors/InteractableActor/BP_ActivasionArtifact.BP_ActivasionArtifact_C"))) (`self.bCanBeActivated`))))

(fn `UserConstructionScript`)