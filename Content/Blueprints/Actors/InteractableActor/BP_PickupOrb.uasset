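; BP_PickupOrb is an interactable orb pickup that credits the first player state with a looted orb.
; It builds on a parent interactable, brightening its point light from the stored default intensity as interaction progress updates arrive.
; On activation it sends the looted-orb message and expires almost immediately via a short life span.
; Stopping interaction before activation also stops its interact and emissive material components.
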(event `self.ReceiveBeginPlay`
  (`parent.ReceiveBeginPlay`)
  (add `self.ObjectActivated` (delegate `ObjectActivated_Event`))
  (set `self.DefaultLightIntensity` (`LightComponentBase.Intensity` (`self.PointLight`)))
  (add `self.UpdateInteract` (delegate `UpdateInteract_Event`)))

(event `UpdateInteract_Event` :!signature `self.UpdateInteract`
  (params (Percent :type "Float (double-precision)"))
  (`LightComponent.SetIntensity` (`self.PointLight`) (* (* (+ Percent 1.0) 1.0) (`self.DefaultLightIntensity`))))

(event `ObjectActivated_Event`
  (message `PlayerStateInterface.AddLootedOrb` (`GameplayStatics.GetPlayerState` 0) 1)
  (`self.SetLifeSpan` 0.1))

(event `/Game/Blueprints/Interfaces/BPI_Interactable.StopInteract`
  (`parent.StopInteract`)
  (if (not (`self.bActivated`))
    (`/Game/Blueprints/Components/C-InteractComponent.StopInteracting` (`self.C-InteractComponent`))
    (`/Game/Blueprints/Components/C-EmissiveMaterialComponent.StopInteracting` (`self.C-EmissiveMaterialComponent`))))

(fn `Interacting`
  (params (UpdateRate :type "Float (double-precision)"))
  (returns (InteractActor :type "Actor Object Reference") (bInRange :type Boolean))
  (bind (_interactactor _binrange) (`parent.Interacting` UpdateRate))
  (return _interactactor _binrange))

(fn `UserConstructionScript`
  (`parent.UserConstructionScript`))