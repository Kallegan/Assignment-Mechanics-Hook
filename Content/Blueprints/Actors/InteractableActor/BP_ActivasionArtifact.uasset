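; Interactable altar artifact that, once activated, spends the player's looted orbs and opens a linked door.
; It stays unactivatable until HighlightAltar enables it and raises its light.
; Activation kills the light, spawns visual orbs that a timeline moves along a spline, spaced by index and wrapping at the end.
; A one-time handler also clears the orb count, messages the trigger actor to open the door and destroys all MechanicsProjectile actors.
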(event `self.ReceiveBeginPlay`
  (`parent.ReceiveBeginPlay`)
  (add `self.ObjectActivated` (delegate `ObjectActivated_Event`))
  (`TimelineComponent.SetPlayRate` (`self.Timeline`) (/ 1.0 (`self.SplineLoopTime`)))
  (set `self.bCanBeActivated` false))

(event `ObjectActivated_Event`
  (bind (_returnvalue_location _returnvalue_rotation) (`KismetMathLibrary.BreakTransform` (`self.GetTransform`)))
  (bind _projectiles (`self.Projectiles`))
  (`LightComponent.SetIntensity` (`self.PointLight`) 0.0)
  (for _ (range 3)
    (`GameplayStatics.PlaySound2D` "/Engine/VREditor/Sounds/UI/Scaling_Up.Scaling_Up" 1.0 1.0 0.0 null null)
    (bind _returnvalue (`|SpawnActorFromClass` "/Game/Blueprints/Actors/BP_VisualPlayerOrb.BP_VisualPlayerOrb_C" (`KismetMathLibrary.MakeTransform` _returnvalue_location _returnvalue_rotation (2.0 2.0 2.0)) "Undefined" "MultiplyWithRoot" null null))
    (`KismetArrayLibrary.Array_AddUnique` (`self.Projectiles`) _returnvalue))
  (`|ExecutionSequence`
    (:`then_0`
      (`self.HandleActivasion`)
      (bind (_direction _movetrack) (`Timeline|Timeline` :!via `PlayFromStart`)
        (:`Update`
          (if (> (`KismetArrayLibrary.Array_Length` _projectiles) 0)
            (for (_array_element _array_index) _projectiles
              (bind _output_get (set `self.DistanceAlongSpline` (+ (`KismetMathLibrary.Lerp` 0.0 (`SplineComponent.GetSplineLength` (`self.Spline`)) _movetrack) (* _array_index (`self.ActorOffset`)))))
              (if (> _output_get (`SplineComponent.GetSplineLength` (`self.Spline`)))
                (set `self.DistanceAlongSpline` (- (`self.DistanceAlongSpline`) (`SplineComponent.GetSplineLength` (`self.Spline`)))))
              (`self.K2_SetActorLocation` _array_element (`SplineComponent.GetLocationAtDistanceAlongSpline` (`self.Spline`) (`self.DistanceAlongSpline`) "World") false false))))))))

(event `HighlightAltar`
  (set `self.bCanBeActivated` true)
  (`LightComponent.SetIntensity` (`self.PointLight`) 24.0))

(fn `HandleActivasion`
  (bind _returnvalue (`GameplayStatics.GetPlayerState` 0))
  (`/Engine/EditorBlueprintResources/StandardMacros.DoOnce` false
    (:`Completed`
      (bind _returnvalue_2 (message `PlayerStateInterface.GetLootedOrbs` _returnvalue))
      (for _ (range _returnvalue_2)
        (message `PlayerStateInterface.RemoveLootedOrb` _returnvalue 1))
      (message `/Game/Blueprints/Interfaces/BPI_Door.OpenDoor` (`self.TriggerActorRef`) 0)
      (bind _outactors (`GameplayStatics.GetAllActorsOfClass` "/Script/Mechanics.MechanicsProjectile"))
      (for _array_element _outactors
        (`self.K2_DestroyActor` _array_element)))))

(fn `Interacting`
  (params (UpdateRate :type "Float (double-precision)"))
  (returns (InteractActor :type "Actor Object Reference") (bInRange :type Boolean))
  (bind (_interactactor _binrange) (`parent.Interacting` UpdateRate))
  (return _interactactor _binrange))

(fn `UserConstructionScript`
  (`parent.UserConstructionScript`))