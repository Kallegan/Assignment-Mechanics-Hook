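; Interactable moving platform that starts moving when its attached-projectile event fires, parenting the projectile to itself with collision disabled.
; Tick interpolates it with sweep toward a first offset, switches to a slower move toward a second offset when close, then destroys the actor on arrival.
; Without a valid game mode, the construction script places goal preview meshes at the offsets and labels text renders with digits from the actor's name.
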(event `self.ReceiveBeginPlay`
  (bind _output_get (set `self.StartLocation` (`self.K2_GetActorLocation`)))
  (set `self.EndLocation` (+ _output_get (`self.EndPosOffset`)))
  (set `self.EndLocation2` (+ _output_get (`self.EndPosOffset2`)))
  (set `self.InterpSpeed` 1.0)
  (set `self.TargetLocation` (`self.EndLocation`)))

(event `self.ReceiveTick`
  (params (DeltaSeconds :type "Float (single-precision)"))
  (bind _returnvalue (`self.K2_GetActorLocation`))
  (if (`self.bShouldMove`)
    (`self.K2_SetActorLocation` (`KismetMathLibrary.VInterpTo` (`self.K2_GetActorLocation`) (`self.TargetLocation`) DeltaSeconds (`self.InterpSpeed`)) true)
    (bind _output_get (set `self.bShouldMove` (and (!= (`self.TargetLocation`) _returnvalue :`ErrorTolerance` 1.0) (!= _returnvalue (`self.EndLocation2`) :`ErrorTolerance` 2.0))))
    (if _output_get
      (if (== (`self.K2_GetActorLocation`) (`self.TargetLocation`) :`ErrorTolerance` 10.0)
        (set `self.TargetLocation` (`self.EndLocation2`))
        (set `self.InterpSpeed` 0.5))
      (else
        (`self.K2_DestroyActor`)))))

(event `self.ProjectAttachedChanged`
  (params (bAttachedProjectile :type Boolean))
  (set `self.bShouldMove` true)
  (bind _projectileref (`self.ProjectileRef`)
    (:`then`
      (`self.K2_AttachToActor` _projectileref self "None" "KeepWorld" "KeepWorld" "KeepWorld" false)
      (`self.SetActorEnableCollision` _projectileref false))
    (:`else`)))

(fn `Interacting`
  (params (UpdateRate :type "Float (double-precision)"))
  (returns (InteractActor :type "Actor Object Reference") (bInRange :type Boolean))
  (return null false))

(fn `UserConstructionScript`
  (locals (NumberString :type String))
  (bind _staticmeshgoal (`self.StaticMeshGoal`))
  (bind _staticmeshgoal1 (`self.StaticMeshGoal1`))
  (`/Engine/EditorBlueprintResources/StandardMacros.IsValid` (`GameplayStatics.GetGameMode`)
    (:`Is Not Valid`
      (`|ExecutionSequence`
        (:`then_0`
          (`SceneComponent.SetWorldScale3D` _staticmeshgoal (`SceneComponent.K2_GetComponentScale` (`self.StaticMesh`)))
          (`SceneComponent.K2_AddWorldOffset` _staticmeshgoal (`self.EndPosOffset`) false true)
          (for _array_element (`KismetStringLibrary.GetCharacterArrayFromString` (`KismetSystemLibrary.GetDisplayName` self))
            (if (`KismetStringLibrary.IsNumeric` _array_element)
              (set `local.NumberString` (`KismetStringLibrary.Concat_StrStr` (`local.NumberString`) _array_element))))
          (`TextRenderComponent.K2_SetText` (`self.TextRender`) (`KismetTextLibrary.Conv_StringToText` (`local.NumberString`)))
          (`TextRenderComponent.K2_SetText` (`self.TextRender1`) (`KismetTextLibrary.Conv_StringToText` (`local.NumberString`)))
          (`TextRenderComponent.K2_SetText` (`self.TextRender2`) (`KismetTextLibrary.Conv_StringToText` (`local.NumberString`))))
        (:`then_1`
          (`SceneComponent.SetWorldScale3D` _staticmeshgoal1 (`SceneComponent.K2_GetComponentScale` (`self.StaticMesh`)))
          (`SceneComponent.K2_AddWorldOffset` _staticmeshgoal1 (`self.EndPosOffset2`) false true))))))