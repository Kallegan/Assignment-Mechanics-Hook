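; An interactable moving platform that travels to an offset end position while a projectile is attached and returns to its start when it is not.
; Attachment changes set the target and attach the referenced projectile to the platform, then Tick eases toward it with VInterpTo at an offset-scaled speed.
; With no game mode, the construction script previews the goal mesh at the offset and labels the platform with digits from its display name.
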(event `self.ReceiveBeginPlay`
  (bind _endposoffset (`self.EndPosOffset`))
  (bind _output_get (set `self.StartLocation` (`self.K2_GetActorLocation`)))
  (set `self.EndLocation` (+ _output_get _endposoffset))
  (set `self.InterpSpeed` (/ (`KismetMathLibrary.VSize` _endposoffset) 300.0)))

(event `self.ReceiveTick`
  (params (DeltaSeconds :type "Float (single-precision)"))
  (if (`self.bShouldMove`)
    (`self.K2_SetActorLocation` (`KismetMathLibrary.VInterpTo` (`self.K2_GetActorLocation`) (`self.TargetLocation`) DeltaSeconds (`self.InterpSpeed`)))
    (set `self.bShouldMove` (!= (`self.TargetLocation`) (`self.K2_GetActorLocation`) :`ErrorTolerance` 1.0))))

(event `self.ProjectAttachedChanged`
  (params (bAttachedProjectile :type Boolean))
  (bind _output_get (set `self.TargetLocation` (`KismetMathLibrary.SelectVector` (`self.EndLocation`) (`self.StartLocation`) bAttachedProjectile)))
  (set `self.bShouldMove` (!= _output_get (`self.K2_GetActorLocation`) :`ErrorTolerance` 0.1))
  (bind _projectileref (`self.ProjectileRef`)
    (:`then`
      (`self.K2_AttachToActor` _projectileref self "None" "KeepWorld" "KeepWorld" "KeepWorld" false))
    (:`else`)))

(fn `Interacting`
  (params (UpdateRate :type "Float (double-precision)"))
  (returns (InteractActor :type "Actor Object Reference") (bInRange :type Boolean))
  (return null false))

(fn `UserConstructionScript`
  (locals (NumberString :type String))
  (bind _staticmeshgoal (`self.StaticMeshGoal`))
  (`/Engine/EditorBlueprintResources/StandardMacros.IsValid` (`GameplayStatics.GetGameMode`)
    (:`Is Not Valid`
      (`SceneComponent.SetWorldScale3D` _staticmeshgoal (`SceneComponent.K2_GetComponentScale` (`self.StaticMesh`)))
      (`SceneComponent.K2_AddWorldOffset` _staticmeshgoal (`self.EndPosOffset`) false false)
      (for _array_element (`KismetStringLibrary.GetCharacterArrayFromString` (`KismetSystemLibrary.GetDisplayName` self))
        (if (`KismetStringLibrary.IsNumeric` _array_element)
          (set `local.NumberString` (`KismetStringLibrary.Concat_StrStr` (`local.NumberString`) _array_element))))
      (`TextRenderComponent.K2_SetText` (`self.TextRender`) (`KismetTextLibrary.Conv_StringToText` (`local.NumberString`)))
      (`TextRenderComponent.K2_SetText` (`self.TextRender1`) (`KismetTextLibrary.Conv_StringToText` (`local.NumberString`))))))