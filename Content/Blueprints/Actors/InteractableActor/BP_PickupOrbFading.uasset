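; Interactable pickup orb actor with a flickering point light and timed, one-shot activation.
; When triggered, it waits a short random delay, then loops a flicker timeline with randomized intensity.
; Each loop raises a capped multiplier that scales light intensity and attenuation radius, so the glow grows stronger despite the "Fading" name.
; Interacting polls the interact component and activates once the in-range timer expires, if activatable.
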(event `/Game/Blueprints/Interfaces/BPI_TriggerActor.TriggerActorEvent`
  (bind _pointlight (`self.PointLight`))
  (bind _increase (`self.Increase`))
  (`|ExecutionSequence`
    (:`then_0`
      (set `self.BaseRadius` (`LocalLightComponent.AttenuationRadius` (`self.PointLight`)))
      (`KismetSystemLibrary.Delay` (`KismetMathLibrary.RandomFloatInRange` 0.1 0.3))
      (bind (_direction _newtrack_0) (`Timeline|LightFlicker` :!via `PlayFromStart` :!label _label)
        (:`Update`
          (bind _output_get (set `self.NewVar` (* _newtrack_0 (`KismetMathLibrary.RandomFloatInRange` 2.0 3.0))))
          (`LightComponent.SetIntensity` _pointlight (* _output_get _increase))
          (`LocalLightComponent.SetAttenuationRadius` _pointlight (* (`self.BaseRadius`) _increase)))
        (:`Finished`
          (set `self.Increase` (`KismetMathLibrary.FClamp` (+ (`self.Increase`) 5.0) 0.0 20.0))
          (goto _label :!via `PlayFromStart`))))))

(event `self.ObjectActivated_Event`
  (`parent.ObjectActivated_Event`))

(fn `Interacting`
  (params (UpdateRate :type "Float (double-precision)"))
  (returns (InteractActor :type "Actor Object Reference") (bInRange :type Boolean))
  (bind (_binrange _percent _timeremaining) (`/Game/Blueprints/Components/C-InteractComponent.UpdateInteracting` (`self.C-InteractComponent`) UpdateRate))
  (set `self.LocalPercent` _percent)
  (if (and _binrange (not (`self.bActivated`)))
    (if (<= _timeremaining 0.0)
      (if (`self.IsActivatable`)
        (set `self.bActivated` true)
        (`self.ObjectActivated`))
      (return self true))
    (else
      (`/Game/Blueprints/Interfaces/BPI_Interactable.StopInteract`)
      (return null false))))

(fn `UserConstructionScript`
  (`parent.UserConstructionScript`))