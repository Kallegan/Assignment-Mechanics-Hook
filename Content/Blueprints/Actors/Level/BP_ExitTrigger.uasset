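; BP_ExitTrigger is a level actor that moves itself like a timed exit door: toward a goal location, then back.
; TriggerActorEvent fires once through a DoOnce and plays a slowed timeline that teleports the actor toward GoalLocation.
; After a fixed delay it stops that timeline and plays a second one back to the location saved at BeginPlay.
; Each update lerps from the current location, so movement compounds rather than following the curve directly.
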(event `self.ReceiveBeginPlay`
  (set `self.StartLocation` (`self.K2_GetActorLocation`)))

(event `/Game/Blueprints/Interfaces/BPI_TriggerActor.TriggerActorEvent`
  (`/Engine/EditorBlueprintResources/StandardMacros.DoOnce` false
    (:`Completed`
      (`|ExecutionSequence`
        (:`then_0`
          (`TimelineComponent.SetPlayRate` (`self.Timeline`) 0.03)
          (bind (_direction _opendoor) (`Timeline|Timeline` :!via `PlayFromStart`)
            (:`Update`
              (`self.K2_SetActorLocation` (`KismetMathLibrary.VLerp` (`self.K2_GetActorLocation`) (`self.GoalLocation`) _opendoor) false true))))
        (:`then_1`
          (`KismetSystemLibrary.Delay` 15.0)
          (`TimelineComponent.Stop` (`self.Timeline`))
          (`TimelineComponent.SetPlayRate` (`self.Timeline_0`) 0.03)
          (bind (_direction_2 _opendoor_2) (`Timeline|Timeline_0` :!via `PlayFromStart`)
            (:`Update`
              (`self.K2_SetActorLocation` (`KismetMathLibrary.VLerp` (`self.K2_GetActorLocation`) (`self.StartLocation`) _opendoor_2) false true))))))))

(fn `UserConstructionScript`)