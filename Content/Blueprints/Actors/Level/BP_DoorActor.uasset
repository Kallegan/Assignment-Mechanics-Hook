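; Level door actor that slides 300 units down to open and returns to its start position when a Character enters its box trigger.
; OpenDoor fires only once through a DoOnce and flags the door open; the overlap then calls CloseDoor and clears the flag.
; Slowed timelines lerp from the current location toward each target, with delayed, pitched-down stone impact sounds and timed stops.
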(event `self.ReceiveBeginPlay`
  (bind _returnvalue (`self.K2_GetActorLocation`))
  (set `self.StartLocation` _returnvalue)
  (set `self.GoalLocation` (+ _returnvalue (0.0 0.0 -300.0))))

(event `/Game/Blueprints/Interfaces/BPI_Door.OpenDoor`
  (params (RoomIndex :type Integer))
  (`/Engine/EditorBlueprintResources/StandardMacros.DoOnce` false
    (:`Completed`
      (`|ExecutionSequence`
        (:`then_0`
          (`TimelineComponent.SetPlayRate` (`self.Timeline`) 0.03)
          (bind (_direction _opendoor) (`Timeline|Timeline` :!via `PlayFromStart`)
            (:`Update`
              (`self.K2_SetActorLocation` (`KismetMathLibrary.VLerp` (`self.K2_GetActorLocation`) (`self.GoalLocation`) _opendoor) false true))))
        (:`then_1`
          (`KismetSystemLibrary.Delay` 1.3)
          (`GameplayStatics.PlaySoundAtLocation` "/Game/SFX/592581__newlocknew__stone-slab-impactwith-a-crunch_217lrs.592581__newlocknew__stone-slab-impactwith-a-crunch_217lrs" (`self.K2_GetActorLocation`) (struct) 0.5 0.7 0.0 null null null null)
          (`KismetSystemLibrary.Delay` 0.5)
          (`TimelineComponent.Stop` (`self.Timeline`))
          (set `self.bOpen` true))))))

(event `CloseDoor`
  (`TimelineComponent.SetPlayRate` (`self.Timeline_0`) 0.2)
  (`|ExecutionSequence`
    (:`then_0`
      (bind (_direction _opendoor) (`Timeline|Timeline_0` :!via `PlayFromStart`)
        (:`Update`
          (`self.K2_SetActorLocation` (`KismetMathLibrary.VLerp` (`self.K2_GetActorLocation`) (`self.StartLocation`) _opendoor) false true))))
    (:`then_1`
      (`KismetSystemLibrary.Delay` 0.5)
      (`GameplayStatics.PlaySoundAtLocation` "/Game/SFX/592581__newlocknew__stone-slab-impactwith-a-crunch_217lrs.592581__newlocknew__stone-slab-impactwith-a-crunch_217lrs" (`self.K2_GetActorLocation`) (struct) 0.75 0.5 0.0 null null null null)
      (`KismetSystemLibrary.Delay` 0.5)
      (`TimelineComponent.Stop` (`self.Timeline`)))))

(event `self.Box.OnComponentBeginOverlap`
  (params (OverlappedComponent :type "PrimitiveComponent Object Reference") (OtherActor :type "Actor Object Reference") (OtherComp :type "PrimitiveComponent Object Reference") (OtherBodyIndex :type Integer) (bFromSweep :type Boolean) (SweepResult :type "HitResult Structure (by ref)"))
  (if (`GameplayStatics.ObjectIsA` OtherActor "/Script/Engine.Character")
    (if (`self.bOpen`)
      (`self.CloseDoor`)
      (set `self.bOpen` false))))

(fn `UserConstructionScript`)