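; Actor component that drives the glow of its owner's static mesh to show hover, interaction and activation states.
; On BeginPlay it puts a dynamic material instance on slot 0, and its events then set that instance's "Alpha" scalar.
; Interaction progress scales the glow; reaching full progress triggers a brief bright flash before the activated level.
; That completion flash sits behind a DoOnce that is never reset.
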(event `self.ReceiveBeginPlay`
  (bind _returnvalue (`Actor.GetComponentByClass` (`self.GetOwner`) "/Script/Engine.StaticMeshComponent"))
  (bind _returnvalue_2 (`PrimitiveComponent.CreateDynamicMaterialInstance` _returnvalue 0 (`self.SourceMaterial`) "None"))
  (bind _output_get (set `self.MaterialInstance` _returnvalue_2))
  (`PrimitiveComponent.SetMaterial` _returnvalue 0 _output_get)
  (`MaterialInstanceDynamic.SetScalarParameterValue` _returnvalue_2 "Alpha" (`self.BaseEmissive`)))

(event `Interacting`
  (params (Alpha :type "Float (double-precision)"))
  (if (< Alpha 1.0)
    (`MaterialInstanceDynamic.SetScalarParameterValue` (`self.MaterialInstance`) "Alpha" (+ (* (`self.InteractingEmissiveMultiplier`) Alpha) (`self.BaseEmissive`)))
    (else
      (`/Engine/EditorBlueprintResources/StandardMacros.DoOnce` false
        (:`Completed`
          (`MaterialInstanceDynamic.SetScalarParameterValue` (`self.MaterialInstance`) "Alpha" 100.0)
          (`KismetSystemLibrary.Delay` 0.1)
          (`self.SetActivated`))))))

(event `StopInteracting`
  (`MaterialInstanceDynamic.SetScalarParameterValue` (`self.MaterialInstance`) "Alpha" (`self.BaseEmissive`)))

(event `SetActivated`
  (`MaterialInstanceDynamic.SetScalarParameterValue` (`self.MaterialInstance`) "Alpha" (`self.ActivatedEmissive`)))

(event `SetDeactivated`
  (`MaterialInstanceDynamic.SetScalarParameterValue` (`self.MaterialInstance`) "Alpha" (`self.BaseEmissive`)))

(event `SetHovered`
  (params (bHovered :type Boolean))
  (`MaterialInstanceDynamic.SetScalarParameterValue` (`self.MaterialInstance`) "Alpha" (`KismetMathLibrary.SelectFloat` (`self.HoveredEmissive`) (`self.BaseEmissive`) bHovered)))