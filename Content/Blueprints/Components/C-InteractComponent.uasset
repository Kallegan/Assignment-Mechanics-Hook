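; Actor component that tracks a timed, hold-to-interact countdown on an interactable object.
; UpdateInteracting subtracts the caller's update rate from the remaining time and returns it with a clamped 0–1 progress and whether the owner is within max range of player 0's pawn.
; StopInteracting resets the countdown to the full interaction time, as does BeginPlay; the component never ticks the timer itself.
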(event `self.ReceiveBeginPlay`
  (set `self.CurrentInteractionTime` (`self.InteractionTime`)))

(fn `StopInteracting`
  (set `self.CurrentInteractionTime` (`self.InteractionTime`)))

(fn `UpdateInteracting`
  (params (UpdateRate :type "Float (double-precision)"))
  (returns (bInRange :type Boolean) (Percent :type "Float (double-precision)") (TimeRemaining :type "Float (double-precision)"))
  (locals (LocalInRange :type Boolean))
  (set `local.LocalInRange` (<= (`Actor.GetDistanceTo` (`self.GetOwner`) (`GameplayStatics.GetPlayerPawn` 0)) (`self.InteractMaxRange`)))
  (bind _output_get (set `self.CurrentInteractionTime` (- (`self.CurrentInteractionTime`) UpdateRate)))
  (return (`local.LocalInRange`) (`KismetMathLibrary.FClamp` (+ (* (/ (`self.CurrentInteractionTime`) (`self.InteractionTime`)) -1.0) 1.0)) _output_get))